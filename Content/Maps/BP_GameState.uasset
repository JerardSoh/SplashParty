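; Game state for a two-team Potatoes versus Beets match, holding team rosters and scores.
; Each team join counts a selection, and MatchCanStart is set once everyone has chosen and the GameInstance's player maximum is reached.
; Multicast-named countdown events forward start and expiry to the local character; the start also turns Beets players around after a short delay.
; GetTeam always returns Potatoes.
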(event Custom|AddPlayerToTeamPotatoes
  (params (Player :type BP%20Player%20State%20Object%20Reference%20%28by%20ref%29))
  (Utilities|Array|Add (Variables|Default|GetPlayersTeamPotatoes) Player)
  (CallFunction|PlayerSelectedTeam))

(event Custom|AddPlayerToTeamBeets
  (params (Player :type BP%20Player%20State%20Object%20Reference%20%28by%20ref%29))
  (Utilities|Array|Add (Variables|Default|GetPlayersTeamBeets) Player)
  (CallFunction|PlayerSelectedTeam))

(event Custom|OnCountdownExpiredMulticast
  (bind _asbp_third_person_character (Utilities|Casting|CastToBP_ThirdPersonCharacter (Pawn|GetControlledPawn (Game|GetPlayerController 0))))
  (Default|OnCountdownExpiredClient _asbp_third_person_character))

(event Custom|PlayerSelectedTeam
  (bind _playerarray (Variables|Default|GetPlayerArray))
  (bind _returnvalue (Utilities|Array|Length _playerarray))
  ;[1 1 1] If all the players have selected the team, the match can start
  (bind _result (Math|Integer|IncrementInt (Variables|Default|GetNumHaveSelectedTeam))
    (:%20%20
      (if (>= _result _returnvalue)
        (bind _asbp_game_instance (Utilities|Casting|CastToBP_GameInstance (Game|GetGameInstance)))
        (if (>= _returnvalue (Variables|/Game/Blueprints/BP_GameInstance.BP_GameInstance_C|GetMaxNumOfPlayers _asbp_game_instance))
          (Variables|Default|SetMatchCanStart? true))))))

(event Custom|StartCountdownMulticast
  (bind _asbp_third_person_character (Utilities|Casting|CastToBP_ThirdPersonCharacter (Pawn|GetControlledPawn (Game|GetPlayerController 0))))
  (Default|StartCountdownClient _asbp_third_person_character)
  (CallFunction|ChangeStartDirection))

(event Custom|ChangeStartDirection
  (CallFunction|ChangeStartDirectionMulti))

(event Custom|ChangeStartDirectionMulti
  (bind _returnvalue (Game|GetPlayerController 0))
  (bind _team (Class|BPIGameInterface|GetTeam(Message) (Variables|/Script/Engine.Controller|GetPlayerState _returnvalue)))
  (switch Utilities|FlowControl|Switch|SwitchonBP_Teams _team
    (:NewEnumerator1
      (Utilities|FlowControl|Delay 1.2)
      (Pawn|SetControlRotation _returnvalue (Math|Rotator|MakeRotator 0.0 0.0 1.8e+02)))))

(event EventIncrementTeamScore
  (params (Team :type BP_Teams%20Enum :default "NewEnumerator0"))
  (switch Utilities|FlowControl|Switch|SwitchonBP_Teams Team
    (:NewEnumerator0
      (Math|Integer|IncrementInt (Variables|Default|GetTeamPotatoesScore)))
    (:NewEnumerator1
      (Math|Integer|IncrementInt (Variables|Default|GetTeamBeetsScore)))))

(fn ConstructionScript)

(fn GetTeamScores
  (return (Variables|Default|GetTeamPotatoesScore) (Variables|Default|GetTeamBeetsScore)))

(fn GetTeam
  (return "NewEnumerator0"))