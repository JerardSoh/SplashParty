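; Character Blueprint for a sad character in the game-end ceremony, playing sad animations with a team-specific look.
; PlayGameEndAnimation, started from the construction script, plays a random montage from SadAnimationArray, waits for its length, then calls itself to loop indefinitely.
; ChangeMeshMaterial sets the mesh's first material slot according to whether the team is Potatoes or Beets.
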(event Custom|ChangeMeshMaterial
  (params (Team :type BP_Teams%20Enum :default "NewEnumerator0"))
  (switch Utilities|FlowControl|Switch|SwitchonBP_Teams Team
    (:NewEnumerator0
      (Rendering|Material|SetMaterial (Variables|Character|GetMesh) 0 "/Game/FallGuysCharacter/CH_FallGuy_MAT.CH_FallGuy_MAT"))
    (:NewEnumerator1
      (Rendering|Material|SetMaterial (Variables|Character|GetMesh) 0 "/Game/FallGuysCharacter/CH_FallGuy_MAT2.CH_FallGuy_MAT2"))))

(event Custom|Play%20Game%20End%20Animation
  (bind _returnvalue (Animation|PlayAnimMontage (Utilities|Array|Get(acopy) (Variables|Default|GetSadAnimationArray) (Math|Random|RandomIntegerinRange 0 3)) 1.0 "None"))
  (Utilities|FlowControl|Delay _returnvalue)
  (CallFunction|PlayGameEndAnimation))

(fn ConstructionScript
  (CallFunction|PlayGameEndAnimation))