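; Game state for a Potatoes versus Beets team match, tracking rosters, scores and start readiness.
; Team picks set MatchCanStart once all present players have picked and the game instance's player maximum is met.
; A score reaching five times the player count stores the winner in BP_GameInstance and triggers ServerTravel.
; Multicast-named events relay countdown start and expiry to the local character, rotating it to its team-tagged start after a delay.
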(event Custom|AddPlayerToTeamPotatoes
  (params (Player :type BP%20Player%20State%20Object%20Reference%20%28by%20ref%29))
  (Utilities|Array|Add (Variables|Default|GetPlayersTeamPotatoes) Player)
  (CallFunction|PlayerSelectedTeam))

(event Custom|AddPlayerToTeamBeets
  (params (Player :type BP%20Player%20State%20Object%20Reference%20%28by%20ref%29))
  (Utilities|Array|Add (Variables|Default|GetPlayersTeamBeets) Player)
  (CallFunction|PlayerSelectedTeam))

(event Custom|OnCountdownExpiredMulticast
  (bind _asbp_third_person_character (Utilities|Casting|CastToBP_ThirdPersonCharacter (Pawn|GetControlledPawn (Game|GetPlayerController 0))))
  (Default|OnCountdownExpiredClient _asbp_third_person_character))

(event Custom|PlayerSelectedTeam
  (bind _playerarray (Variables|Default|GetPlayerArray))
  (bind _returnvalue (Utilities|Array|Length _playerarray))
  ;[1 1 1] If all the players have selected the team, the match can start
  (bind _result (Math|Integer|IncrementInt (Variables|Default|GetNumHaveSelectedTeam))
    (:%20%20
      (if (>= _result _returnvalue)
        (bind _asbp_game_instance (Utilities|Casting|CastToBP_GameInstance (Game|GetGameInstance)))
        (if (>= _returnvalue (Variables|/Game/Blueprints/BP_GameInstance.BP_GameInstance_C|GetMaxNumOfPlayers _asbp_game_instance))
          (Variables|Default|SetMatchCanStart? true))))))

(event Custom|StartCountdownMulticast
  (bind _asbp_third_person_character (Utilities|Casting|CastToBP_ThirdPersonCharacter (Pawn|GetControlledPawn (Game|GetPlayerController 0))))
  (Default|StartCountdownClient _asbp_third_person_character)
  (CallFunction|ChangeStartDirection))

(event Custom|ChangeStartDirection
  (CallFunction|ChangeStartDirectionMulti))

(event Custom|ChangeStartDirectionMulti
  (bind _returnvalue (Game|GetPlayerController 0))
  (bind _returnvalue_2 (Pawn|GetControlledPawn _returnvalue))
  (bind _team (Class|BPIGameInterface|GetTeam(Message) (Variables|/Script/Engine.Controller|GetPlayerState _returnvalue)))
  (switch Utilities|FlowControl|Switch|SwitchonBP_Teams _team
    (:NewEnumerator0
      (bind _outactors (Actor|GetAllActorsOfClasswithTag 0 "Potatoes"))
      (Utilities|FlowControl|Delay 3.0)
      (Pawn|SetControlRotation _returnvalue (Transformation|GetActorRotation (Utilities|Array|Get(acopy) _outactors)))
      (Transformation|SetActorRotation _returnvalue_2 (Transformation|GetActorRotation (Utilities|Array|Get(acopy) _outactors))))
    (:NewEnumerator1
      (bind _outactors_2 (Actor|GetAllActorsOfClasswithTag "/Script/Engine.PlayerStart" "Beets"))
      (Utilities|FlowControl|Delay 3.0)
      (Pawn|SetControlRotation _returnvalue (Transformation|GetActorRotation (Utilities|Array|Get(acopy) _outactors_2)))
      (Transformation|SetActorRotation _returnvalue_2 (Transformation|GetActorRotation (Utilities|Array|Get(acopy) _outactors_2))))))

(event EventIncrementTeamScore
  (params (Team :type BP_Teams%20Enum :default "NewEnumerator0"))
  (bind _playerarray (Variables|Default|GetPlayerArray))
  (bind _returnvalue (Utilities|Array|Length _playerarray))
  (bind _returnvalue_2 (* _returnvalue 5))
  (switch Utilities|FlowControl|Switch|SwitchonBP_Teams Team
    (:NewEnumerator0
      (bind _result (Math|Integer|IncrementInt (Variables|Default|GetTeamPotatoesScore))
        (:%20%20
          _)))
    (:NewEnumerator1
      (bind _result_2 (Math|Integer|IncrementInt (Variables|Default|GetTeamBeetsScore))
        (:%20%20
          _))))
  (if (>= _result _returnvalue_2)
    (bind _asbp_game_instance (Utilities|Casting|CastToBP_GameInstance (Game|GetGameInstance)))
    (Variables|/Game/Blueprints/BP_GameInstance.BP_GameInstance_C|SetBlue%20Won _asbp_game_instance true)
    (bind _assplash_party_game_mode (Utilities|Casting|CastToSplashPartyGameMode (Game|GetGameMode) :!label _label))
    (Default|ServerTravel _assplash_party_game_mode)
    (elif (>= _result_2 _returnvalue_2)
      (bind _asbp_game_instance_2 (Utilities|Casting|CastToBP_GameInstance (Game|GetGameInstance)))
      (Variables|/Game/Blueprints/BP_GameInstance.BP_GameInstance_C|SetBlue%20Won _asbp_game_instance_2 false)
      (goto _label))))

(fn ConstructionScript)

(fn GetTeamScores
  (return (Variables|Default|GetTeamPotatoesScore) (Variables|Default|GetTeamBeetsScore)))

(fn GetTeam
  (return "NewEnumerator0"))