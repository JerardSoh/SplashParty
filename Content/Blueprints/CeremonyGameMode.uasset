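; Game mode for the post-match ceremony that spawns a happy or sad character for each starting player, based on team and result.
; HandleStartingNewPlayer calls SpawnPlayer, which reads the team from PlayerState and advances that team's counter to pick a tagged PlayerStart.
; The game instance's BlueWon flag selects the Potatoes or Beets character class; spawned characters are not possessed here.
; GetTeamScores and GetTeam return only fixed placeholder values.
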(event EventBeginPlay)

(event EventSpawnPlayer
  (params (PlayerController :type Player%20Controller%20Object%20Reference))
  (bind _next_index_blue (Variables|Default|GetNext%20Index%20Blue))
  (bind _next_index_pink (Variables|Default|GetNext%20Index%20Pink))
  (bind _team (Class|BPIGameInterface|GetTeam(Message) (Variables|/Script/Engine.Controller|GetPlayerState PlayerController)))
  (switch Utilities|FlowControl|Switch|SwitchonBP_Teams _team
    (:NewEnumerator0
      (Math|Integer|IncrementInt _next_index_blue
        (:%20%20
          (bind _outactors (Actor|GetAllActorsOfClasswithTag "/Script/Engine.PlayerStart" "Potatoes"))
          (bind _asbp_game_instance (Utilities|Casting|CastToBP_GameInstance (Game|GetGameInstance)))
          (if (Variables|/Game/Blueprints/BP_GameInstance.BP_GameInstance_C|GetBlue%20Won _asbp_game_instance)
            (Game|SpawnActorfromClass "/Game/Maps/BP_CeremonyHappyCharacter.BP_CeremonyHappyCharacter_C" (Math|Transform|MakeTransform (Transformation|GetActorLocation (Utilities|Array|Get(acopy) _outactors _next_index_blue)) (Transformation|GetActorRotation (Utilities|Array|Get(acopy) _outactors _next_index_blue))) "Undefined" 0 0)
            (else
              (Game|SpawnActorfromClass "/Game/Maps/BP_CeremonySadCharacter1.BP_CeremonySadCharacter1_C" (Math|Transform|MakeTransform (Transformation|GetActorLocation (Utilities|Array|Get(acopy) _outactors _next_index_blue)) (Transformation|GetActorRotation (Utilities|Array|Get(acopy) _outactors _next_index_blue))) "Undefined" 0 0))))))
    (:NewEnumerator1
      (Math|Integer|IncrementInt _next_index_pink
        (:%20%20
          (bind _outactors_2 (Actor|GetAllActorsOfClasswithTag "/Script/Engine.PlayerStart" "Beets"))
          (bind _asbp_game_instance_2 (Utilities|Casting|CastToBP_GameInstance (Game|GetGameInstance)))
          (if (Variables|/Game/Blueprints/BP_GameInstance.BP_GameInstance_C|GetBlue%20Won _asbp_game_instance_2)
            (Game|SpawnActorfromClass "/Game/Maps/BP_CeremonySadCharacter1_Child.BP_CeremonySadCharacter1_Child_C" (Math|Transform|MakeTransform (Transformation|GetActorLocation (Utilities|Array|Get(acopy) _outactors_2 _next_index_pink)) (Transformation|GetActorRotation (Utilities|Array|Get(acopy) _outactors_2 _next_index_pink))) "Undefined" 0 0)
            (else
              (Game|SpawnActorfromClass "/Game/Maps/BP_CeremonyHappyCharacter_Child.BP_CeremonyHappyCharacter_Child_C" (Math|Transform|MakeTransform (Transformation|GetActorLocation (Utilities|Array|Get(acopy) _outactors_2 _next_index_pink)) (Transformation|GetActorRotation (Utilities|Array|Get(acopy) _outactors_2 _next_index_pink))) "Undefined" 0 0))))))))

(event EventHandleStartingNewPlayer
  (params (NewPlayer :type Player%20Controller%20Object%20Reference))
  (CallFunction|SpawnPlayer NewPlayer))

(event EventTick
  (params (DeltaSeconds :type Float%20%28single-precision%29)))

(fn ConstructionScript)

(fn GetTeamScores
  (return 0 0))

(fn GetTeam
  (return "NewEnumerator0"))