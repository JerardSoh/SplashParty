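; Game mode for the two-team Splash Party match, Potatoes versus Beets, handling player spawning and the opening countdown.
; Each new player gets a third-person character at a random PlayerStart tagged with their team, with location and rotation drawn by separate random picks.
; Shortly after BeginPlay, a five-second server timer starts, and the GameState multicasts countdown start and expiry.
; GetTeamScores and GetTeam only return fixed placeholder values.
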(event Custom|StartCountdownServer
  (Utilities|Time|SetTimerbyEvent (delegate Custom|OnCountdownExpired) 5.0)
  (bind _asbp_game_state (Utilities|Casting|CastToBP_GameState (Game|GetGameState)))
  (Default|StartCountdownMulticast _asbp_game_state))

(event Custom|OnCountdownExpired
  (bind _asbp_game_state (Utilities|Casting|CastToBP_GameState (Game|GetGameState)))
  (Default|OnCountdownExpiredMulticast _asbp_game_state))

(event EventHandleStartingNewPlayer
  (params (NewPlayer :type Player%20Controller%20Object%20Reference))
  (CallFunction|SpawnPlayer NewPlayer))

(event EventSpawnPlayer
  (params (PlayerController :type Player%20Controller%20Object%20Reference))
  (bind _team (Class|BPIGameInterface|GetTeam(Message) (Variables|/Script/Engine.Controller|GetPlayerState PlayerController)))
  (switch Utilities|FlowControl|Switch|SwitchonBP_Teams _team
    (:NewEnumerator0
      (Variables|Default|SetTagName "Potatoes"))
    (:NewEnumerator1
      (Variables|Default|SetTagName "Beets")))
  (bind _outactors (Actor|GetAllActorsOfClasswithTag "/Script/Engine.PlayerStart" (Variables|Default|GetTagName)))
  (bind _returnvalue (Game|SpawnActorfromClass "/Game/Blueprints/BP_ThirdPersonCharacter.BP_ThirdPersonCharacter_C" (Math|Transform|MakeTransform (Transformation|GetActorLocation (.OutItem (Utilities|Array|Random _outactors))) (Transformation|GetActorRotation (.OutItem (Utilities|Array|Random _outactors)))) "AdjustIfPossibleButAlwaysSpawn" 0 0))
  (Pawn|Possess PlayerController _returnvalue))

(event EventBeginPlay
  (Utilities|FlowControl|Delay 1.0)
  (CallFunction|StartCountdownServer))

(fn ConstructionScript)

(fn GetTeamScores
  (return 0 0))

(fn GetTeam
  (return "NewEnumerator0"))